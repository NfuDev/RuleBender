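; BenderGameInstance is a game instance Blueprint that handles level progression and restarts.
; GotoNextLevel increments CurrentLevelIndex, clamps it to the BenderLevels array bounds and opens that level by object reference, so the last level reloads instead of wrapping.
; RestartLevel reopens the active map by its current name, leaving an unconnected open-by-reference node using CurrentLevel that never runs.
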(fn `Goto Next Level`
  (bind _benderlevels (`self.BenderLevels`))
  (bind _currentlevelindex (`self.CurrentLevelIndex`))
  (set `self.CurrentLevelIndex` (`KismetMathLibrary.Clamp` (+ _currentlevelindex 1) 0 (- (`KismetArrayLibrary.Array_Length` _benderlevels) 1)))
  (`GameplayStatics.OpenLevelBySoftObjectPtr` (`|GetArrayItem` _benderlevels _currentlevelindex)))

(fn `RestartLevel`
  (bind _returnvalue (`GameplayStatics.GetCurrentLevelName` true))
  (`GameplayStatics.OpenLevel` (`KismetStringLibrary.Conv_StringToName` _returnvalue)))